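; Child Blueprint of a speed pickup that adds material changes to the inherited pickup behavior.
; On BeginPlay it runs the parent logic, then applies its Material variable to the first slot of its static mesh.
; On Pickup sets that same material on the collecting character's capsule component, not its mesh, before calling the parent pickup logic.
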(event `self.ReceiveBeginPlay`
  (bind _material (`self.material`))
  (`parent.ReceiveBeginPlay`)
  (`PrimitiveComponent.SetMaterial` (`self.StaticMesh_0`) 0 _material)
  (set `self.Material` _material))

(fn `On Pickup`
  (params (Character :type "Character Object Reference") (`Other Actor` :type "/Game/Clint_Work/Hider/Blueprints/BP_Hider Object Reference"))
  (`PrimitiveComponent.SetMaterial` (`Character.CapsuleComponent` Character) 0 (`self.material`))
  (`parent.On Pickup` Character null))

(fn `UserConstructionScript`
  (`parent.UserConstructionScript`))