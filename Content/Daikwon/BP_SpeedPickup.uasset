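; BP_SpeedPickup is a pickup that temporarily changes a BP_Hider's speed when that hider overlaps it.
; On authority only, overlap applies SpeedIncrease through ChangeSpeed, disables collision, waits EffectDuration, reverses the change and destroys the pickup.
; SetActorHiddenInGame is passed false, so the pickup stays visible during the delay.
; A separate OnPickup path sets PlayerSpeed directly, and the overlap event never calls it.
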(event `self.ReceiveBeginPlay`)

(event `self.ReceiveActorBeginOverlap`
  (params (OtherActor :type "Actor Object Reference"))
  (`/Engine/EditorBlueprintResources/ActorMacros.Switch Has Authority`
    (:`Authority`
      (if true
        (bind _asbp_hider (cast `/Game/Clint_Work/Hider/Blueprints/BP_Hider` OtherActor))
        (`/Game/Clint_Work/Hider/Blueprints/BP_Hider.ChangeSpeed` _asbp_hider (`self.SpeedIncrease`))
        (`self.SetActorEnableCollision` false)
        (`self.SetActorHiddenInGame` false)
        (`KismetSystemLibrary.PrintString` "Before speed effect end")
        (`KismetSystemLibrary.Delay` (`self.Effect Duration`))
        (`KismetSystemLibrary.PrintString` "After speed increase end")
        (`/Game/Clint_Work/Hider/Blueprints/BP_Hider.ChangeSpeed` _asbp_hider (* (`self.SpeedIncrease`) -1.0))
        (`self.K2_DestroyActor`)
        (else
          (bind _asbp_hider_2 (cast `/Game/Clint_Work/Hider/Blueprints/BP_Hider` OtherActor))
          (`/Game/Clint_Work/Hider/Blueprints/BP_Hider.ChangeSpeed` _asbp_hider_2 (`self.SpeedIncrease`))
          (`self.SetActorEnableCollision` false)
          (`self.SetActorHiddenInGame` false)
          (`KismetSystemLibrary.PrintString` "Before speed effect end")
          (`KismetSystemLibrary.Delay` (`self.Effect Duration`))
          (`KismetSystemLibrary.PrintString` "After speed increase end")
          (`/Game/Clint_Work/Hider/Blueprints/BP_Hider.ChangeSpeed` _asbp_hider_2 (* (`self.SpeedIncrease`) -1.0))
          (`self.K2_DestroyActor`))))))

(fn `DeactivatePickup`)

(fn `ModifyPlayerSpeed`
  (params (`Other Actor` :type "/Game/Clint_Work/Hider/Blueprints/BP_Hider Object Reference"))
  (locals (NewLocalVar :type "SubmixEffectDelaySettings Structure"))
  (`/Engine/EditorBlueprintResources/ActorMacros.Switch Has Authority`
    (:`Authority`
      (bind _asbp_hider (cast `/Game/Clint_Work/Hider/Blueprints/BP_Hider` `Other Actor`))
      (set `/Game/Clint_Work/Hider/Blueprints/BP_Hider.PlayerSpeed` (`self.SpeedIncrease`) _asbp_hider)
      (`GameplayStatics.GetActorOfClass` "/Game/Clint_Work/Hider/Blueprints/BP_Hider.BP_Hider_C")
      (`SubmixEffectDelayStatics.SetDelayLength` (`self.Delay Settings`) (`self.Effect Duration`))
      (`self.ResetSinglePlayerSpeed` (`self.Target`)))))

(fn `On Pickup`
  (params (Character :type "Character Object Reference") (`Other Actor` :type "/Game/Clint_Work/Hider/Blueprints/BP_Hider Object Reference"))
  (`KismetSystemLibrary.PrintString` "Test Collision")
  (`self.ModifyPlayerSpeed` `Other Actor`)
  (`self.K2_DestroyActor`))

(fn `ResetSinglePlayerSpeed`
  (bind _returnvalue (`GameplayStatics.GetActorOfClass` "/Game/Clint_Work/Hider/Blueprints/BP_Hider.BP_Hider_C"))
  (set `/Game/Clint_Work/Hider/Blueprints/BP_Hider.PlayerSpeed` (`self.BaseSpeed`) _returnvalue))

(fn `UserConstructionScript`)