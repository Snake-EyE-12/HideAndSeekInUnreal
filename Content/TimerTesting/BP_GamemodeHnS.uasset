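; Game mode for a hide-and-seek match with a countdown that decides when the game ends.
; The first player to join possesses a Hider at the first PlayerStart found, and later players possess Seekers at the second.
; A looping one-second timer decrements TimeLeft, whose RepNotify is empty.
; Timeout or a Seeker tag stops the timer and calls OnGameEnd on player pawns, with true for timeout and false for a tag.
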(event `self.ReceiveBeginPlay`
  (bind _returnvalue (`KismetSystemLibrary.K2_SetTimerDelegate` (delegate `TickTimer`) 1.0 true))
  (set `self.SecondTimer` _returnvalue)
  (`self.SetTime` (`self.GameInitTime`)))

(event `TickTimer`
  (`self.RemoveTime` 1))

(event `self.HandleStartingNewPlayer`
  (params (NewPlayer :type "PlayerController Object Reference"))
  (bind _outactors (`GameplayStatics.GetAllActorsOfClass` "/Script/Engine.PlayerStart"))
  (if (== (`self.P1`) 0)
    (bind _result (`/Engine/EditorBlueprintResources/StandardMacros.IncrementInt` (`self.P1`))
      (:`  `
        (set `self.P1` _result)
        (bind _returnvalue (`|SpawnActorFromClass` "/Game/Clint_Work/Hider/Blueprints/BP_Hider.BP_Hider_C" (`self.GetTransform` (`|GetArrayItem` _outactors)) "Undefined" "MultiplyWithRoot" null null))
        (`Controller.Possess` NewPlayer _returnvalue)))
    (else
      (bind _returnvalue_2 (`|SpawnActorFromClass` "/Game/Clint_Work/Seeker/Blueprints/BP_Seeker.BP_Seeker_C" (`self.GetTransform` (`|GetArrayItem` _outactors 1)) "Undefined" "MultiplyWithRoot" null null))
      (`Controller.Possess` NewPlayer _returnvalue_2))))

(fn `AddTime`
  (params (Time :type Integer))
  (`self.SetTime` (+ (`self.TimeLeft`) Time)))

(fn `OnRep_TimeLeft`)

(fn `OnSeekerTagHider`
  (`KismetSystemLibrary.PrintString` "Game Over")
  (`KismetSystemLibrary.K2_ClearAndInvalidateTimerHandle` (`self.SecondTimer`))
  (for _array_element (`GameStateBase.PlayerArray` (`GameplayStatics.GetGameState`))
    (bind _asbp_third_person_character_timer_test (cast `/Game/TimerTesting/BP_ThirdPersonCharacterTimerTest` (`PlayerState.GetPawn` _array_element)))
    (`/Game/TimerTesting/BP_ThirdPersonCharacterTimerTest.OnGameEnd` _asbp_third_person_character_timer_test false)))

(fn `OnTimerReachZero`
  (`KismetSystemLibrary.PrintString` "Game Over")
  (for _array_element (`GameStateBase.PlayerArray` (`GameplayStatics.GetGameState`))
    (bind _asbp_third_person_character_timer_test (cast `/Game/TimerTesting/BP_ThirdPersonCharacterTimerTest` (`PlayerState.GetPawn` _array_element)))
    (`/Game/TimerTesting/BP_ThirdPersonCharacterTimerTest.OnGameEnd` _asbp_third_person_character_timer_test true)))

(fn `RemoveTime`
  (params (Time :type Integer))
  (`self.SetTime` (- (`self.TimeLeft`) Time)))

(fn `SetTime`
  (params (Time :type Integer))
  (bind _output_get (set `self.TimeLeft` Time))
  (if (<= _output_get 0)
    (`self.OnTimerReachZero`)
    (`KismetSystemLibrary.K2_ClearAndInvalidateTimerHandle` (`self.SecondTimer`))))

(fn `UserConstructionScript`)